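; BP_FRecoverable is a clamped float value that refills over time to MaxValue.
; SetValue clamps and broadcasts the raw and clamped values, starting recovery automatically at zero when AutoRecover is set.
; TryRecover converts the current Value into elapsed time and opens a Tick gate, so partial refills keep the same linear rate.
; Tick lerps Value until RecoverTime, then closes the gate and snaps to max, without broadcasting changes.
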(event Custom|SetValue
  (params (NewValue :type Float%20%28double-precision%29))
  (bind _output_get (Variables|Default|SetValue (Math|Float|Clamp(Float) NewValue 0.0 (Variables|Default|GetMaxValue))))
  (Utilities|FlowControl|Sequence
    (:then_0
      (if (and (Variables|Default|GetAutoRecover) (<= _output_get 0.0))
        (CallFunction|TryRecover)))
    (:then_1
      (Default|CallOnSetValue NewValue _output_get))))

(event Custom|TryRecover
  (Variables|Default|SetTime (Math|Float|Lerp 0.0 (Variables|Default|GetRecoverTime) (Math|Float|NormalizetoRange (Variables|Default|GetValue) 0.0 (Variables|Default|GetMaxValue))))
  (Utilities|FlowControl|Gate true) ; enters at Open
)

(event EventBeginPlay)

(event EventTick
  (params (DeltaSeconds :type Float%20%28single-precision%29))
  (Utilities|FlowControl|Sequence
    (:then_1
      (Utilities|FlowControl|Gate true :!label _label
        (:Exit
          (if (<= (+ DeltaSeconds (Variables|Default|GetTime)) (Variables|Default|GetRecoverTime))
            (bind _output_get (Variables|Default|SetTime (+ DeltaSeconds (Variables|Default|GetTime))))
            (Variables|Default|SetValue (Math|Float|Lerp 0.0 (Variables|Default|GetMaxValue) (Math|Float|NormalizetoRange _output_get 0.0 (Variables|Default|GetRecoverTime))))
            (else
              (Utilities|FlowControl|Sequence
                (:then_0
                  (goto _label Close))
                (:then_1
                  (Variables|Default|SetValue (Variables|Default|GetMaxValue)))))))))))